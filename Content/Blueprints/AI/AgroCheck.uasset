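; AgroCheck is a behavior tree tick Blueprint, likely a service, that detects targets for ARPGAI-controlled enemies.
; It caches the controller, then sphere-traces around its pawn for chosen object types, ignoring all ARPGAI_Character actors.
; Each hit gets a Camera-channel line-of-sight trace, setting TargetToFollow and TargetLocation when visible, or clearing only TargetToFollow when blocked.
; The loop never breaks, so the last hit decides TargetToFollow, and zero hits leave it unchanged.
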(event `self.ReceiveTick`
  (params (OwnerActor :type "Actor Object Reference") (DeltaSeconds :type "Float (single-precision)"))
  (bind _returnvalue (`Actor.K2_GetActorLocation` (`Controller.K2_GetPawn` (`self.ARPGEnemy_Ref`))))
  (if (not (!= (`self.ARPGEnemy_Ref`) null))
    (bind _asarpgai (cast `/Game/Blueprints/AI/ARPGAI` OwnerActor))
    (set `self.ARPGEnemy_Ref` _asarpgai))
  (bind _outactors (`GameplayStatics.GetAllActorsOfClass` "/Game/Blueprints/AI/ARPGAI_Character.ARPGAI_Character_C"))
  (set `self.MyLocation` _returnvalue)
  (bind _outhits (`KismetSystemLibrary.SphereTraceMultiForObjects` _returnvalue (+ _returnvalue (0.0 0.0 15.0)) 1500.0 (`self.DesiredObejctTypes`) false _outactors))
  (for _array_element _outhits
    (bind (_bblockinghit _binitialoverlap _time _distance _location _impactpoint _normal _impactnormal _physmat _hitactor) (`GameplayStatics.BreakHitResult` _array_element))
    (bind _outhit (`KismetSystemLibrary.LineTraceSingle` (`self.MyLocation`) (`Actor.K2_GetActorLocation` _hitactor) "TraceTypeQuery2" false _outactors))
    (bind (_bblockinghit_2 _binitialoverlap_2 _time_2 _distance_2 _location_2 _impactpoint_2 _normal_2 _impactnormal_2 _physmat_2 _hitactor_2) (`GameplayStatics.BreakHitResult` _outhit))
    (if (== _hitactor_2 _hitactor)
      (`BTFunctionLibrary.SetBlackboardValueAsObject` (`self.TargetToFollow`) _hitactor_2)
      (`BTFunctionLibrary.SetBlackboardValueAsVector` (`self.TargetLocation`) (`Actor.K2_GetActorLocation` _hitactor_2))
      (else
        (`BTFunctionLibrary.SetBlackboardValueAsObject` (`self.TargetToFollow`))))))