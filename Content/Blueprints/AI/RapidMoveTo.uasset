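; RapidMoveTo is a Behavior Tree task that moves an AI-controlled enemy pawn toward a blackboard target actor.
; On execute, it casts the owner to ARPGAI, caches that reference, and runs AIMoveTo on its pawn with a small acceptance radius.
; A successful move finishes the task as failed; a failed move or failed cast never calls FinishExecute.
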(event `self.ReceiveExecute`
  (params (OwnerActor :type "Actor Object Reference"))
  (if (not (!= (`self.ARPGEnemy_Ref`) null))
    (bind _asarpgai (cast `/Game/Blueprints/AI/ARPGAI` OwnerActor))
    (set `self.ARPGEnemy_Ref` _asarpgai))
  (`|AIMoveTo` (`Controller.K2_GetPawn` (`self.ARPGEnemy_Ref`)) (0.0 0.0 0.0) (`BTFunctionLibrary.GetBlackboardValueAsActor` (`self.TargetToFollow`)) 50.0 true
    (:`OnSuccess`
      (`self.FinishExecute` false))))